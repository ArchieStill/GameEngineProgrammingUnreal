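; Base pickupable item actor that tallies collected items in four color categories: blue, red, green and yellow.
; Its Pickup event destroys the actor, then switches on ItemType to call the matching CountManager counter and play that color's 2D sound, printing "failed" for unknown types.
; The construction script caches the CountManager reference through GetActorOfClass.
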(event `/Game/GEP/Blueprints/Interfaces/BPI_Pickupable.Pickup`
  (bind _countmanager (`self.CountManager`))
  (`self.K2_DestroyActor`)
  (switch `int` (`self.ItemType`)
    (:`Default`
      (`KismetSystemLibrary.PrintString` "failed"))
    (:`1`
      (`/Game/GEP/Blueprints/Items/CountManager.BlueCount` _countmanager)
      (`GameplayStatics.PlaySound2D` "/Game/GEP/Sounds/Pickup/BluePickupSound.BluePickupSound" 1.0 1.0 0.0 null null))
    (:`2`
      (`/Game/GEP/Blueprints/Items/CountManager.RedCount` _countmanager)
      (`GameplayStatics.PlaySound2D` "/Game/GEP/Sounds/Pickup/RedPickupSound.RedPickupSound" 1.0 1.0 0.0 null null))
    (:`3`
      (`/Game/GEP/Blueprints/Items/CountManager.GreenCount` _countmanager)
      (`GameplayStatics.PlaySound2D` "/Game/GEP/Sounds/Pickup/GreenPickupSound.GreenPickupSound" 1.0 1.0 0.0 null null))
    (:`4`
      (`/Game/GEP/Blueprints/Items/CountManager.YellowCount` _countmanager)
      (`GameplayStatics.PlaySound2D` "/Game/GEP/Sounds/Pickup/YellowPickupSound.YellowPickupSound" 1.0 1.0 0.0 null null))))

(fn `UserConstructionScript`
  (bind _returnvalue (`GameplayStatics.GetActorOfClass` "/Game/GEP/Blueprints/Items/CountManager.CountManager_C"))
  (set `self.CountManager` _returnvalue))