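; CountManager is an item-side actor Blueprint that keeps per-color score tallies for blue, red, green and yellow.
; Each color has its own function, BlueCount, RedCount, GreenCount or YellowCount, which adds one to that color's score variable.
; The event graph and construction script are empty, so the counts change only when those functions are called externally.
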(fn `BlueCount`
  (bind _output_get (set `self.BlueScore` (+ (`self.BlueScore`) 1))))

(fn `GreenCount`
  (bind _output_get (set `self.GreenScore` (+ (`self.GreenScore`) 1))))

(fn `RedCount`
  (bind _output_get (set `self.RedScore` (+ (`self.RedScore`) 1))))

(fn `UserConstructionScript`)

(fn `YellowCount`
  (bind _output_get (set `self.YellowScore` (+ (`self.YellowScore`) 1))))