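; ChangeSelected is an actor Blueprint that tracks which of four colored items (blue, red, green, yellow) the player has selected.
; Its construction script caches the BP_PlayerCharacter found in the level.
; ChangeSelectedItem switches on that character's ChosenItem, setting the matching visibility variable to Visible and the other three to Hidden.
; The event graph is empty, and nothing in this asset calls the function or reads those variables.
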(fn `Change Selected Item`
  (switch `int` (`/Game/GEP/Blueprints/Essentials/BP_PlayerCharacter.ChosenItem` (`self.Player`))
    (:`1`
      (set `self.BlueVisible` "Visible")
      (set `self.RedVisible` "Hidden")
      (set `self.GreenVisible` "Hidden")
      (set `self.YellowVisible` "Hidden"))
    (:`2`
      (set `self.RedVisible` "Visible")
      (set `self.BlueVisible` "Hidden")
      (set `self.GreenVisible` "Hidden")
      (set `self.YellowVisible` "Hidden"))
    (:`3`
      (set `self.GreenVisible` "Visible")
      (set `self.BlueVisible` "Hidden")
      (set `self.RedVisible` "Hidden")
      (set `self.YellowVisible` "Hidden"))
    (:`4`
      (set `self.YellowVisible` "Visible")
      (set `self.BlueVisible` "Hidden")
      (set `self.RedVisible` "Hidden")
      (set `self.GreenVisible` "Hidden"))))

(fn `UserConstructionScript`
  (bind _returnvalue (`GameplayStatics.GetActorOfClass` "/Game/GEP/Blueprints/Essentials/BP_PlayerCharacter.BP_PlayerCharacter_C"))
  (set `self.Player` _returnvalue))